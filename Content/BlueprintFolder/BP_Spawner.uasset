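; BP_Spawner is an actor that keeps spawning AI enemies while the level holds fewer BP_SurvivalCharacter actors than AmountToSpawn.
; Each Tick counts those actors and, when short, runs a random Delay between the minimum and maximum times.
; It then spawns a random EnemyClass pawn with the EnemyAI behavior tree at a random point inside its Box, with NoCollisionFail enabled.
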(event `self.ReceiveTick`
  (params (DeltaSeconds :type "Float (single-precision)"))
  (bind _box (`self.Box`))
  (bind _outactors (`GameplayStatics.GetAllActorsOfClass` "/Game/BlueprintFolder/BP_SurvivalCharacter.BP_SurvivalCharacter_C"))
  (if (< (`KismetArrayLibrary.Array_Length` _outactors) (`self.AmountToSpawn`))
    (`KismetSystemLibrary.Delay` (`KismetMathLibrary.Conv_IntToDouble` (`KismetMathLibrary.RandomIntegerInRange` (`self.MinimumDelayTime`) (`self.MaximumDelayTime`))))
    (`AIBlueprintHelperLibrary.SpawnAIFromClass` (`KismetArrayLibrary.Array_Random` (`self.EnemyClass`)) (`self.EnemyAI`) (`KismetMathLibrary.RandomPointInBoundingBox` (`SceneComponent.K2_GetComponentLocation` _box) (`BoxComponent.BoxExtent` _box)) (struct) true null)))

(fn `UserConstructionScript`)