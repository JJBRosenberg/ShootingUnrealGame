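; Player character Blueprint that handles looking at and interacting with objects, plus pausing the game.
; Each Tick traces from the actor along the camera's forward vector, storing the hit actor and adding a new door prompt widget whenever it is a BP_InteractDoor.
; Interact calls InteractWithObject on a stored BP_Interaction and removes door prompts.
; PauseGame toggles pause via FlipFlop, while E only fires a debug-drawn camera trace.
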(event `Key|E`
  (params (Key :type "Key Structure"))
  (bind _camera (`self.Camera`))
  (bind _returnvalue (`SceneComponent.K2_GetComponentLocation` _camera))
  (:`Pressed`
    (bind _outhit (`KismetSystemLibrary.LineTraceSingle` :`Start` _returnvalue :`End` (+ (* (`SceneComponent.GetForwardVector` _camera) 300.0) _returnvalue) :`TraceChannel` "TraceTypeQuery1" :`DrawDebugType` "ForDuration" :`DrawTime` 1.0))))

(event `InputAction|Interact`
  (params (Key :type "Key Structure"))
  (:`Pressed`
    (bind _asbp_interaction (cast `/Game/BlueprintFolder/BP_Interaction` (`self.ObjectLookingAt`)))
    (`/Game/BlueprintFolder/BP_Interaction.InteractWithObject` _asbp_interaction)
    (bind _foundwidgets (`WidgetBlueprintLibrary.GetAllWidgetsOfClass` "/Game/UI/WBP_DoorInteract.WBP_DoorInteract_C"))
    (`Widget.RemoveFromParent` _foundwidgets)))

(event `self.ReceiveTick`
  (params (DeltaSeconds :type "Float (single-precision)"))
  (bind _returnvalue (`self.K2_GetActorLocation` self))
  (bind (_outhit _returnvalue_2) (`KismetSystemLibrary.LineTraceSingle` _returnvalue (+ _returnvalue (* (`SceneComponent.GetForwardVector` (`self.Camera`)) (`self.ForwardDistance`))) "TraceTypeQuery1"))
  (if _returnvalue_2
    (bind _output_get (set `self.ObjectLookingAt` (`.HitActor` (`GameplayStatics.BreakHitResult` _outhit))))
    (bind _asbp_interact_door (cast `/Game/BlueprintFolder/BP_InteractDoor` _output_get))
    (if (== _asbp_interact_door (`self.ObjectLookingAt`))
      (bind _returnvalue_3 (`|CreateWidget` "/Game/UI/WBP_DoorInteract.WBP_DoorInteract_C"))
      (`UserWidget.AddToViewport` _returnvalue_3 0))
    (else
      (set `self.ObjectLookingAt` null))))

(event `InputAction|PauseGame` :paused true
  (params (Key :type "Key Structure"))
  (:`Pressed`
    (`/Engine/EditorBlueprintResources/StandardMacros.FlipFlop`
      (:`A`
        (`GameplayStatics.SetGamePaused` true))
      (:`B`
        (`GameplayStatics.SetGamePaused` false)))))

(fn `UserConstructionScript`
  (`parent.UserConstructionScript`))